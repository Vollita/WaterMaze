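; BP_AI is an AI-controlled pawn that detects the player and can perform a melee attack animation.
; Its PawnSensing component sets the seeingPlayer blackboard key to true when it sees a pawn tagged Player; this graph never clears it.
; The AttrackPlayer event plays a push-shove montage on the mesh, using the Attracking flag to block re-entry until the montage completes.
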(event OnSeePawn(PawnSensing)
  (params (Pawn :type Pawn%20Object%20Reference))
  ;[0.15 0.15 0.15 0.5] 当AI感知到标签为Play的Pawn时，就把AI Controller里的黑板组件中的seeingPlayer设置为布尔值（可以在行为树中将是否设置seeingPlayer为布尔值进行执行哪些任务的判断）
  ;;[0.15 0.15 0.15 0.5] 当AI感知到某个Pawn时（前面给AI加了一个感知器））
  (if (Actor|ActorHasTag Pawn "Player")
    ;;[0.15 0.15 0.15 0.5] （如果AI感知到 即true）将某个键的值设置为布尔值，这里是seeingPlayer
    (AI|Components|Blackboard|SetValueasBool (AI|GetBlackboard (AI|GetAIController self)) (Utilities|Name|MakeLiteralName "seeingPlayer") true)))

(event Custom|Attrack%20Player
  ;[0.15 0.15 0.15 0.5] BP_AI的Attrack Payer事件。如果没有攻击，就设定attracking为是然后执行一次攻击的蒙太奇动画，然后再把attracking设置为否
  (if (not (Variables|Default|Getattracking?))
    (Variables|Default|Setattracking? true)
    (Animation|Montage|PlayMontage (Variables|Character|GetMesh) "/Game/AI/Paired_PushShove_Att_Montage.Paired_PushShove_Att_Montage"
      (:OnCompleted
        (Variables|Default|Setattracking? false)))))

(event EventBeginPlay)

(event Collision|EventActorBeginOverlap
  (params (OtherActor :type Actor%20Object%20Reference)))

(event EventTick
  (params (DeltaSeconds :type Float%20%28single-precision%29)))

(fn ConstructionScript)